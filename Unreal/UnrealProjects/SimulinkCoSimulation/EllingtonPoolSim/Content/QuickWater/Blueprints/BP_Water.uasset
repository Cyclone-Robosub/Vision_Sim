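; Configurable water volume actor with a surface plane, underwater post-processing and underwater sound, built entirely in the Construction Script.
; PostProcessBox's X/Y extent and Depth size and place both boxes and the non-spatialized sound's box attenuation.
; Dynamic materials share absorption, scattering and caustic settings between the plane and post-process blendables, which also receive the plane's world height.
; The event graph, including AudioBox overlaps, has no logic.
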(event `self.AudioBox.OnComponentBeginOverlap`
  (params (OverlappedComponent :type "PrimitiveComponent Object Reference") (OtherActor :type "Actor Object Reference") (OtherComp :type "PrimitiveComponent Object Reference") (OtherBodyIndex :type Integer) (bFromSweep :type Boolean) (SweepResult :type "HitResult Structure (by ref)")))

(event `self.AudioBox.OnComponentEndOverlap`
  (params (OverlappedComponent :type "PrimitiveComponent Object Reference") (OtherActor :type "Actor Object Reference") (OtherComp :type "PrimitiveComponent Object Reference") (OtherBodyIndex :type Integer)))

(fn `UserConstructionScript`
  (bind (_fogambient_r _fogambient_g _fogambient_b) (break `LinearColor` (`self.FogAmbient`)))
  (bind (_waterlinecolor_r _waterlinecolor_g _waterlinecolor_b) (break `LinearColor` (`self.WaterlineColor`)))
  (bind _sound (`self.Sound`))
  (bind _postprocessbox (`self.PostProcessBox`))
  (bind _audiobox (`self.AudioBox`))
  (bind _depth (`self.Depth`))
  (bind (_scattering_r _scattering_g _scattering_b) (break `LinearColor` (`self.Scattering`)))
  (bind _returnvalue (`KismetMathLibrary.MakeColor` _scattering_r _scattering_g _scattering_b (`self.ScatterOpacity`)))
  (bind (_returnvalue_x _returnvalue_y _returnvalue_z) (`KismetMathLibrary.BreakVector` (`SceneComponent.K2_GetComponentLocation` (`self.Water Plane`))))
  (bind (_returnvalue_x_2 _returnvalue_y_2) (`KismetMathLibrary.BreakVector` (`BoxComponent.GetUnscaledBoxExtent` (`self.PostProcessBox`))))
  (bind (_returnvalue_x_3 _returnvalue_y_3) (`KismetMathLibrary.BreakVector` (`BoxComponent.GetScaledBoxExtent` (`self.PostProcessBox`))))
  (bind _returnvalue_2 (* (`self.Depth`) -1.0))
  (bind _linearcolor (make `LinearColor` (`self.AbsorptionR`) (`self.AbsorptionG`) (`self.AbsorptionB`)))
  (bind (_relativelocation_x _relativelocation_y) (`KismetMathLibrary.BreakVector` (`SceneComponent.RelativeLocation` (`self.AudioBox`))))
  (bind _returnvalue_3 (`KismetMathLibrary.MakeVector` _relativelocation_x _relativelocation_y (- _returnvalue_2 15.0)))
  (`BoxComponent.SetBoxExtent` _audiobox (`KismetMathLibrary.MakeVector` _returnvalue_x_2 _returnvalue_y_2 (+ _depth 15.0)) true)
  (`BoxComponent.SetBoxExtent` _postprocessbox (`KismetMathLibrary.MakeVector` _returnvalue_x_2 _returnvalue_y_2 (+ _depth 30.0)) true)
  (`SceneComponent.K2_SetRelativeLocation` _postprocessbox (`KismetMathLibrary.MakeVector` _relativelocation_x _relativelocation_y _returnvalue_2) false false)
  (`SceneComponent.K2_SetRelativeLocation` _audiobox _returnvalue_3 false false)
  (`AudioComponent.SetSound` (`self.Sound`) (`self.UnderwaterSound`))
  (set `AudioComponent.AttenuationOverrides` (make `SoundAttenuationSettings` :`bSpatialize` false :`AttenuationShape` "Box" :`AttenuationShapeExtents` (`KismetMathLibrary.MakeVector` _returnvalue_x_3 _returnvalue_y_3 (+ (`self.Depth`) 15.0)) :`FalloffDistance` 5.0) _sound)
  (`SceneComponent.K2_SetRelativeLocation` _sound _returnvalue_3 false false)
  ;[1 1 1] Caustics
  (bind _returnvalue_4 (`KismetMaterialLibrary.CreateDynamicMaterialInstance` (`self.UnderwaterPostCaustics`)))
  (`MaterialInstanceDynamic.SetScalarParameterValue` _returnvalue_4 "WaterHeight" _returnvalue_z)
  (`MaterialInstanceDynamic.SetScalarParameterValue` _returnvalue_4 "Caustic Brightness" (`self.CausticBrightness`))
  (`MaterialInstanceDynamic.SetScalarParameterValue` _returnvalue_4 "Caustic Size" (`self.CausticTiling`))
  (`MaterialInstanceDynamic.SetScalarParameterValue` _returnvalue_4 "Caustics Fade In Distance" (`self.CausticFadeInDistance`))
  (`PostProcessComponent.AddOrUpdateBlendable` (`self.PostProcess`) _returnvalue_4 1.0)
  ;[1 1 1] Fog/Absorption
  (bind _returnvalue_5 (`KismetMaterialLibrary.CreateDynamicMaterialInstance` (`self.UnderwaterPost`)))
  (`MaterialInstanceDynamic.SetScalarParameterValue` _returnvalue_5 "WaterHeight" _returnvalue_z)
  (`MaterialInstanceDynamic.SetVectorParameterValue` _returnvalue_5 "AbsorptionCoefficents" _linearcolor)
  (`MaterialInstanceDynamic.SetVectorParameterValue` _returnvalue_5 "Fog Scatter Color" _returnvalue)
  (`MaterialInstanceDynamic.SetScalarParameterValue` _returnvalue_5 "Scattering Aniso" (`self.Anisotropy`))
  (`MaterialInstanceDynamic.SetScalarParameterValue` _returnvalue_5 "Fog" (`self.FogDensity`))
  (`MaterialInstanceDynamic.SetVectorParameterValue` _returnvalue_5 "Fog Ambient Color" (`KismetMathLibrary.MakeColor` _fogambient_r _fogambient_g _fogambient_b (`self.FogAmbientBrightness`)))
  (`MaterialInstanceDynamic.SetVectorParameterValue` _returnvalue_5 "Band Color" (`KismetMathLibrary.MakeColor` _waterlinecolor_r _waterlinecolor_g _waterlinecolor_b (`self.WaterlineBrightness`)))
  (`PostProcessComponent.AddOrUpdateBlendable` (`self.PostProcess`) _returnvalue_5 1.0)
  ;[1 1 1] Water Plane
  (bind _returnvalue_6 (`PrimitiveComponent.CreateDynamicMaterialInstance` (`self.Water Plane`) 0 (`self.WaterMaterial`) "None"))
  (`MaterialInstanceDynamic.SetVectorParameterValue` _returnvalue_6 "AbsorptionCoefficents" _linearcolor)
  (`MaterialInstanceDynamic.SetVectorParameterValue` _returnvalue_6 "ScatteringCoefficents" _returnvalue)
  (`MaterialInstanceDynamic.SetTextureParameterValue` _returnvalue_6 "NormalMap" (`self.WaterTexture`))
  (`MaterialInstanceDynamic.SetScalarParameterValue` _returnvalue_6 "WaveScale" (`self.Tiling`))
  (`MaterialInstanceDynamic.SetScalarParameterValue` _returnvalue_6 "WaveSpeed" (`self.Speed`))
  (`MaterialInstanceDynamic.SetScalarParameterValue` _returnvalue_6 "WaveStrength" (`self.Strength`))
  (`MaterialInstanceDynamic.SetScalarParameterValue` _returnvalue_6 "Specular" (`self.Specular`))
  (`MaterialInstanceDynamic.SetScalarParameterValue` _returnvalue_6 "Roughness" (`self.Roughness`))
  (`MaterialInstanceDynamic.SetScalarParameterValue` _returnvalue_6 "ScatteringAnisotropy" (`self.Anisotropy`))
  (`MaterialInstanceDynamic.SetScalarParameterValue` _returnvalue_6 "Caustic Brightness" (`self.CausticBrightness`))
  (`MaterialInstanceDynamic.SetScalarParameterValue` _returnvalue_6 "Caustic Size" (`self.CausticTiling`))
  (`MaterialInstanceDynamic.SetScalarParameterValue` _returnvalue_6 "Caustics Fade In Distance" (`self.CausticFadeInDistance`))
  (`MaterialInstanceDynamic.SetScalarParameterValue` _returnvalue_6 "FogDepth" (`self.FogDepth`))
  (`MaterialInstanceDynamic.SetScalarParameterValue` _returnvalue_6 "FogFadeStrength" (`self.FogFadeStrength`))
  (`MaterialInstanceDynamic.SetVectorParameterValue` _returnvalue_6 "DarkColor" (`self.FogDarkColor`))
  (`MaterialInstanceDynamic.SetVectorParameterValue` _returnvalue_6 "LightColor" (`self.FogLightColor`)))